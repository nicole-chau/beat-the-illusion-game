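; RedLightIcon_BP is an actor that displays a red light icon once the Grid's score is at least 100.
; It hides the RedLightIcon component on BeginPlay.
; Every Tick it looks up the Grid with GetActorOfClass, without caching it, and shows or hides the component according to that score.
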(event `self.ReceiveBeginPlay`
  (`SceneComponent.SetVisibility` (`self.RedLightIcon`) false false))

(event `self.ReceiveTick`
  (params (DeltaSeconds :type "Float (single-precision)"))
  (bind _returnvalue (`GameplayStatics.GetActorOfClass` "/Script/Project5.Grid"))
  (if (>= (`Grid.score` _returnvalue) 100)
    (`SceneComponent.SetVisibility` (`self.RedLightIcon`) true false)
    (else
      (`SceneComponent.SetVisibility` (`self.RedLightIcon`) false false))))

(fn `UserConstructionScript`)