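; Menu actor that spins three shape components, a cylinder, cone and prism, in a stepped rotation.
; Tick rotates all three locally at a constant, frame-rate-independent speed.
; Whenever the cone's world yaw comes within a small tolerance of a quarter turn, the owning actor disables its own tick, waits on a short Delay, then re-enables it.
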(event `self.ReceiveTick`
  (params (DeltaSeconds :type "Float (single-precision)"))
  (bind _returnvalue (`ActorComponent.GetOwner` (`self.cylinder`)))
  (`SceneComponent.K2_AddLocalRotation` (`self.cylinder`) (* (struct :`Yaw` 70.0) DeltaSeconds) false false)
  (`SceneComponent.K2_AddLocalRotation` (`self.cone`) (* (struct :`Yaw` 70.0) DeltaSeconds) false false)
  (`SceneComponent.K2_AddLocalRotation` (`self.prism`) (* (struct :`Yaw` 70.0) DeltaSeconds) false false)
  (if (`KismetMathLibrary.NearlyEqual_FloatFloat` (mod (.yaw (`SceneComponent.K2_GetComponentRotation` (`self.cone`))) 90.0) 0.0 0.5)
    (`self.SetActorTickEnabled` _returnvalue false)
    (`self.SetActorTickEnabled` (`ActorComponent.GetOwner` (`self.cone`)) false)
    (`self.SetActorTickEnabled` (`ActorComponent.GetOwner` (`self.prism`)) false)
    (`KismetSystemLibrary.Delay` 2.0)
    (`self.SetActorTickEnabled` _returnvalue true)
    (`self.SetActorTickEnabled` (`ActorComponent.GetOwner` (`self.cone`)) true)
    (`self.SetActorTickEnabled` (`ActorComponent.GetOwner` (`self.prism`)) true)))

(fn `UserConstructionScript`)